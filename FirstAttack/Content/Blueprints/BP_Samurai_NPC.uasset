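; BP_Samurai_NPC is the computer-controlled samurai in a duel, attacking on its own once the draw phase starts.
; On BeginPlay it runs the parent logic, then binds to the draw-phase-started event on the duel game mode.
; When that event fires, it waits for a delay and then calls Attack, with no Tick logic involved.
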(event Custom|OnDrawPhaseStarted
  (Utilities|FlowControl|Delay (Variables|Default|GetDuration))
  (CallFunction|Attack))

(event EventBeginPlay
  (|CallParentFunction)
  (EventDispatchers|BindEventtoDrawPhaseStarted (Variables|Default|GetAsGMDuel) (delegate Custom|OnDrawPhaseStarted)))

(event Collision|EventActorBeginOverlap
  (params (OtherActor :type Actor%20Object%20Reference)))

(event EventTick
  (params (DeltaSeconds :type Float%20%28single-precision%29))
  (|CallParentFunction DeltaSeconds) ; This node is disabled and will not be called.\nDrag off pins to build functionality.
)

(fn ConstructionScript
  (|CallParentFunction))